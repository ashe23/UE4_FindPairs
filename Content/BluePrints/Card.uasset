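; Clickable card actor for a color-matching memory game, flipped by timelines that swap its material to reveal or hide its color.
; The first click registers the card as MainGameMode's ActiveCard, and a second click on another card compares colors.
; A match increments PairCount and shatters both destructible cards with particles, while a mismatch flips both back.
; Click events are disabled during the result delay, then the game mode checks for game over.
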(event `self.ReceiveBeginPlay`
  (set `PlayerController.bEnableClickEvents` true (`GameplayStatics.GetPlayerController` 0))
  (bind _asmain_game_mode (cast `/Game/BluePrints/MainGameMode` (`GameplayStatics.GetGameMode`)))
  (set `self.MainGameMode` _asmain_game_mode))

(event `self.ReceiveActorOnClicked`
  (params (ButtonPressed :type "Key Structure" :default "AnyKey"))
  (bind _maingamemode (`self.MainGameMode`))
  (`self.setActiveCard`)
  (set `self.CurrentIndex` (`KismetStringLibrary.Conv_StringToInt` (`KismetStringLibrary.GetSubstring` (`KismetSystemLibrary.GetDisplayName` self) 4 2)))
  ;[1 1 1] Checks if currently clicked card is not same as active card
  (if (!= (`/Game/BluePrints/MainGameMode.ActiveCard` (`self.MainGameMode`)) self)
    (`self.Rotate180`)
    ;[1 1 1] Checks if clicked card has same color as active card
    (if (`|EnumEquality` (`/Game/BluePrints/Card.Color` (`/Game/BluePrints/MainGameMode.ActiveCard` (`self.MainGameMode`))) (`self.Color`))
      (`self.DisableClickEvents`)
      (`self.IncrementPairCount`)
      (`KismetSystemLibrary.Delay` 0.9)
      (`GameplayStatics.SpawnSound2D` "/Game/Assets/Audio/TruePair.TruePair")
      (`self.ApplyDamageToBothCards`)
      (else
        (`self.DisableClickEvents`)
        (`KismetSystemLibrary.Delay` 0.9)
        (`GameplayStatics.SpawnSound2D` "/Game/Assets/Audio/FalsePair.FalsePair")
        (`self.Unrotate180`)
        (`self.Unrotate180` (`/Game/BluePrints/MainGameMode.ActiveCard` _maingamemode))))
    (set `/Game/BluePrints/MainGameMode.ActiveCard` null _maingamemode)
    (`self.EnableClickEvents`)
    (`/Game/BluePrints/MainGameMode.isGameOver` _maingamemode)))

(event `Rotate180`
  (bind (_returnvalue_roll _returnvalue_pitch _returnvalue_yaw) (`KismetMathLibrary.BreakRotator` (`self.K2_GetActorRotation`)))
  ;[1 1 1] Rotates card by 180 angle and changes material
  (bind (_direction _rotation) (`Timeline|Timeline_0` :!via `PlayFromStart`)
    (:`Update`
      (`self.K2_SetActorRelativeRotation` (`KismetMathLibrary.MakeRotator` _rotation _returnvalue_pitch _returnvalue_yaw)))
    (:`Finished`
      (set `self.isCardClicked` true)
      (`self.setMaterialBasedOnColor`))))

(event `Unrotate180`
  (bind (_returnvalue_roll _returnvalue_pitch _returnvalue_yaw) (`KismetMathLibrary.BreakRotator` (`self.K2_GetActorRotation`)))
  ;[1 1 1] Unrotating card back to default rotation and making material default
  (bind (_direction _rotation) (`Timeline|Timeline_1` :!via `ReverseFromEnd`)
    (:`Update`
      (`self.K2_SetActorRelativeRotation` (`KismetMathLibrary.MakeRotator` _rotation _returnvalue_pitch _returnvalue_yaw)))
    (:`Finished`
      (`PrimitiveComponent.SetMaterial` (`self.DestructibleComponent`) 0 "/Game/Assets/Materials/M_CardFront.M_CardFront")
      (set `self.isCardClicked` false))))

(event `ApplyDamageToBothCards`
  (bind _activecard (`/Game/BluePrints/MainGameMode.ActiveCard` (`self.MainGameMode`)))
  (bind _destructiblecomponent (`DestructibleActor.DestructibleComponent` _activecard))
  (`ActorComponent.Activate` (`self.ParticleSystem`) false)
  (`DestructibleComponent.ApplyRadiusDamage` (`self.DestructibleComponent`) 100.0 (`self.K2_GetActorLocation`) 100.0 100.0 true)
  (`ActorComponent.Activate` (`/Game/BluePrints/Card.ParticleSystem` _activecard) false)
  (`DestructibleComponent.ApplyRadiusDamage` _destructiblecomponent 100.0 (`SceneComponent.K2_GetComponentLocation` _destructiblecomponent) 100.0 100.0 true))

(fn `DisableClickEvents`
  (set `PlayerController.bEnableClickEvents` false (`GameplayStatics.GetPlayerController` 0)))

(fn `EnableClickEvents`
  (set `PlayerController.bEnableClickEvents` true (`GameplayStatics.GetPlayerController` 0)))

(fn `IncrementPairCount`
  (bind _maingamemode (`self.MainGameMode`))
  (bind _result (`/Engine/EditorBlueprintResources/StandardMacros.IncrementInt` (`/Game/BluePrints/MainGameMode.PairCount` _maingamemode))
    (:`  `
      (set `/Game/BluePrints/MainGameMode.PairCount` _result _maingamemode))))

(fn `setActiveCard`
  (bind _maingamemode (`self.MainGameMode`))
  (if (not (`KismetSystemLibrary.IsValid` (`/Game/BluePrints/MainGameMode.ActiveCard` _maingamemode)))
    (bind _output_get (set `/Game/BluePrints/MainGameMode.ActiveCard` self _maingamemode))
    (`self.Rotate180` _output_get)))

(fn `setMaterialBasedOnColor`
  (bind _destructiblecomponent (`self.DestructibleComponent`))
  (switch `/Game/BluePrints/E_Colors` (`self.Color`)
    (:`NewEnumerator0`
      (`PrimitiveComponent.SetMaterial` _destructiblecomponent 0 "/Game/Assets/Materials/PM_Red.PM_Red"))
    (:`NewEnumerator1`
      (`PrimitiveComponent.SetMaterial` _destructiblecomponent 0 "/Game/Assets/Materials/PM_Green.PM_Green"))
    (:`NewEnumerator2`
      (`PrimitiveComponent.SetMaterial` _destructiblecomponent 0 "/Game/Assets/Materials/PM_Blue.PM_Blue"))
    (:`NewEnumerator3`
      (`PrimitiveComponent.SetMaterial` _destructiblecomponent 0 "/Game/Assets/Materials/PM_Orange.PM_Orange"))))

(fn `UserConstructionScript`)