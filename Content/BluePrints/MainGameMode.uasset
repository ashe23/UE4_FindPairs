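; Game mode for a color card pair-matching game that opens the menu, lays out the cards and handles winning.
; BeginPlay shows the menu and cursor, hides the pawn and calls SpawnCards, which builds a grid with Difficulty rows, each holding every E_Colors value in shuffled order.
; isGameOver checks whether PairCount equals half the cards, then plays a sound, shows the win widget and stores game time as a formatted WinTime.
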(event `self.ReceiveTick`
  (params (DeltaSeconds :type "Float (single-precision)")))

(event `self.ReceiveBeginPlay`
  ;[1 1 1] Show main menu, that asks user to pick dificulty of game
  (bind _returnvalue (`|CreateWidget` "/Game/HUD/Menu.Menu_C"))
  (`UserWidget.AddToViewport` _returnvalue 0)
  (`self.SpawnCards`)
  (set `PlayerController.bShowMouseCursor` true (`GameplayStatics.GetPlayerController` 0))
  (`self.SetActorHiddenInGame` (`GameplayStatics.GetPlayerPawn` 0) true))

(event `isGameOver`
  (if (== (`self.PairCount`) (/ (`KismetArrayLibrary.Array_Length` (`self.Cards`)) 2))
    (`GameplayStatics.PlaySound2D` "/Game/Assets/Audio/positive.positive")
    (bind _returnvalue (`|CreateWidget` "/Game/HUD/YouWonWidget.YouWonWidget_C"))
    (`UserWidget.AddToViewport` _returnvalue 0)
    (set `self.WinTime` (`.Time(M M:SS)` (`self.ConvertTime` (`KismetSystemLibrary.GetGameTimeInSeconds`))))))

(fn `RemoveAllCards`
  (`GameplayStatics.GetAllActorsOfClass` "/Game/BluePrints/Card.Card_C")
  (`self.K2_DestroyActor`))

(fn `SpawnCards`
  (bind _cardspacing (`self.CardSpacing`))
  (bind _colorsarray (`self.ColorsArray`))
  (bind _enumvalue (foreach `/Game/BluePrints/E_Colors`)
    (:`LoopBody`
      (`KismetArrayLibrary.Array_Add` _colorsarray _enumvalue))
    (:`then`
      (for _index (range (`self.Difficulty`))
        (`KismetArrayLibrary.Array_Shuffle` _colorsarray)
        (for _index_2 (range (enumcount `/Game/BluePrints/E_Colors`))
          (bind _returnvalue (`|SpawnActorFromClass` "/Game/BluePrints/Card.Card_C" (`KismetMathLibrary.MakeTransform` (+ (`KismetMathLibrary.MakeVector` (* _index _cardspacing) (* _index_2 _cardspacing) 0.01) (`self.StartingLocation`)) (struct) (1.0 1.0 0.01)) "Undefined" "OverrideRootScale"))
          (set `/Game/BluePrints/Card.Color` (`KismetArrayLibrary.Array_Get` (`self.ColorsArray`) _index_2) _returnvalue)
          (`KismetArrayLibrary.Array_Add` (`self.Cards`) _returnvalue))))))

(fn `UserConstructionScript`)